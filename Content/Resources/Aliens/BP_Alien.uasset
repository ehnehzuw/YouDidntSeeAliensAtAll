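; BP_Alien is an alien actor that plays a dissolve effect on spawn and tracks its distance from the player.
; BeginPlay creates a dynamic instance of Dissolve_Inst on the mesh, and a timeline animates its "Disslove" scalar parameter.
; Tick stores the horizontal distance to the first player's controlled pawn in Distance.
; Code that hands the alien to its UBP_Distance widget is disconnected and never runs.
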(event `self.ReceiveBeginPlay`
  (bind _mesh (`self.Mesh`))
  (`PrimitiveComponent.SetMaterial` (`self.Mesh`) 0 "/Game/Texture/Dissolve_Inst.Dissolve_Inst")
  (bind _returnvalue (`PrimitiveComponent.CreateDynamicMaterialInstance` _mesh 0 (`PrimitiveComponent.GetMaterial` _mesh 0) "None"))
  (bind _output_get (set `self.CubeMaterial` _returnvalue))
  (bind (_direction _newtrack_0) (`Timeline|Timeline` :!via `PlayFromStart`)
    (:`Update`
      (`MaterialInstanceDynamic.SetScalarParameterValue` _output_get "Disslove" (`KismetMathLibrary.Lerp` 1.0 -1.0 _newtrack_0)))))

(event `self.ReceiveTick`
  (params (DeltaSeconds :type "Float (single-precision)"))
  (bind _returnvalue (`Controller.K2_GetPawn` (`GameplayStatics.GetPlayerController` 0)))
  (`/Engine/EditorBlueprintResources/StandardMacros.IsValid` _returnvalue
    (:`Is Valid`
      (set `self.Distance` (`self.GetHorizontalDistanceTo` _returnvalue self)))))

(fn `UserConstructionScript`)
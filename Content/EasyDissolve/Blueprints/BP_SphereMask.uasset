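; BP_SphereMask is an actor that drives a sphere mask through the MPC_SphereMask material parameter collection, apparently for a dissolve effect.
; The construction script writes the Sphere component's location and scale-derived radius into Location_1 and Radius_1.
; Tick rewrites both, incrementing a Scale multiplier every frame, so the radius grows at a frame-rate-dependent speed.
; Timeline movement, opacity fade and actor scaling nodes are unconnected and never run.
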(event `self.ReceiveTick`
  (params (DeltaSeconds :type "Float (single-precision)"))
  (bind _result (`/Engine/EditorBlueprintResources/StandardMacros.IncrementFloat` (`self.scale`))
    (:`  `
      (set `self.scale` _result)
      (`KismetMaterialLibrary.SetScalarParameterValue` "/Game/EasyDissolve/Materials/CollectionParameters/MPC_SphereMask.MPC_SphereMask" "Radius_1" (.x (* (/ (`SceneComponent.K2_GetComponentScale` (`self.Sphere`)) 2.0) (`self.scale`))))
      (`KismetMaterialLibrary.SetVectorParameterValue` "/Game/EasyDissolve/Materials/CollectionParameters/MPC_SphereMask.MPC_SphereMask" "Location_1" (`KismetMathLibrary.Conv_VectorToLinearColor` (`SceneComponent.K2_GetComponentLocation` (`self.Sphere`)))))))

(fn `UserConstructionScript`
  (`KismetMaterialLibrary.SetScalarParameterValue` "/Game/EasyDissolve/Materials/CollectionParameters/MPC_SphereMask.MPC_SphereMask" "Radius_1" (.x (* (/ (`SceneComponent.K2_GetComponentScale` (`self.Sphere`)) 2.0) 100.0)))
  (`KismetMaterialLibrary.SetVectorParameterValue` "/Game/EasyDissolve/Materials/CollectionParameters/MPC_SphereMask.MPC_SphereMask" "Location_1" (`KismetMathLibrary.Conv_VectorToLinearColor` (`SceneComponent.K2_GetComponentLocation` (`self.Sphere`)))))
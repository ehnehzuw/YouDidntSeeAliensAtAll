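; BP_Squid is a grabbable animated squid with a skeletal mesh and a GrabComponent.
; On BeginPlay it plays a one-shot fall-down animation, then after a short delay hands the mesh back to its Animation Blueprint.
; Grab and drop events toggle IsHeld, which is not read in these graphs.
; Dance_1 replays the fall-down animation without restoring Animation Blueprint mode, and Dance_2 is an empty stub.
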(event `self.ReceiveBeginPlay`
  (`SkeletalMeshComponent.PlayAnimation` (`self.Meshy_AI_请根据这个帮我_biped_Character_output`) "/Game/Resources/Meshes/Squid/Animation/Squid_FallDown.Squid_FallDown" false)
  (`KismetSystemLibrary.Delay` 3.0)
  (`SkeletalMeshComponent.SetAnimationMode` (`self.Meshy_AI_请根据这个帮我_biped_Character_output`) "AnimationBlueprint" true))

(event `self.GrabComponent.OnGrabbed`
  (set `self.IsHeld?` true))

(event `self.GrabComponent.OnDropped`
  (set `self.IsHeld?` false))

(event `Dance_1`
  (`SkeletalMeshComponent.PlayAnimation` (`self.Meshy_AI_请根据这个帮我_biped_Character_output`) "/Game/Resources/Meshes/Squid/Animation/Squid_FallDown.Squid_FallDown" false))

(event `Dance_2`)

(fn `UserConstructionScript`)
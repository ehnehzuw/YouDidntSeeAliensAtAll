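; BP_SavedObject is an actor that dissolves in on spawn and can be pinned as a Meta XR spatial anchor.
; On BeginPlay it applies a dissolve material and a Timeline drives the dynamic instance's "Disslove" parameter across its range.
; Pressing the 1 key creates a spatial anchor at the actor's transform, saves it to local storage, then prints the anchor's transform as debug output.
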(event `Key|One`
  (params (Key :type "Key Structure"))
  (:`Pressed`
    (`OculusXRAsyncAction_CreateSpatialAnchor.OculusXRAsyncCreateSpatialAnchor` self (`self.GetTransform`)
      (:`Success`
        (`KismetSystemLibrary.PrintString` "Hello")
        (bind _anchor (`OculusXRAsyncAction_SaveAnchor.OculusXRAsyncSaveAnchor` self "Local")
          (:`Success`
            (bind _outtransform (`OculusXRAnchorBPFunctionLibrary.GetAnchorTransformByHandle` (`OculusXRAnchorComponent.GetHandle` _anchor)))
            (`KismetSystemLibrary.PrintString` (`KismetStringLibrary.Conv_TransformToString` _outtransform))))))))

(event `self.ReceiveBeginPlay`
  (bind _staticmesh (`self.StaticMesh`))
  (`PrimitiveComponent.SetMaterial` _staticmesh 0 "/Game/Texture/Dissolve_Inst.Dissolve_Inst")
  (bind _returnvalue (`PrimitiveComponent.CreateDynamicMaterialInstance` _staticmesh 0 (`PrimitiveComponent.GetMaterial` _staticmesh 0) "None"))
  (bind (_direction _newtrack_0) (`Timeline|Timeline` :!via `PlayFromStart`)
    (:`Update`
      (`MaterialInstanceDynamic.SetScalarParameterValue` _returnvalue "Disslove" (`KismetMathLibrary.Lerp` 1.0 -1.0 _newtrack_0)))))

(fn `UserConstructionScript`)